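; BP_Trace is a short-lived actor that shows a frozen pose snapshot of the player character, like an afterimage.
; On BeginPlay it copies the pose from the first skeletal mesh component of player 0's BP_ThirdPersonCharacter onto its Body mesh.
; It reveals Body after a brief delay, then hides it and destroys itself ten seconds later.
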(event `self.ReceiveBeginPlay`
  (bind _asbp_third_person_character (cast `/Game/ThirdPerson/Blueprints/BP_ThirdPersonCharacter` (`GameplayStatics.GetPlayerCharacter` 0)))
  (`PoseableMeshComponent.CopyPoseFromSkeletalComponent` (`self.body`) (`|GetArrayItem` (`self.K2_GetComponentsByClass` _asbp_third_person_character "/Script/Engine.SkeletalMeshComponent")))
  (`KismetSystemLibrary.Delay` 0.01)
  (`SceneComponent.SetVisibility` (`self.body`) true false)
  (`KismetSystemLibrary.Delay` 10.0)
  (`SceneComponent.SetVisibility` (`self.body`) false false)
  (`self.K2_DestroyActor`))

(fn `UserConstructionScript`)