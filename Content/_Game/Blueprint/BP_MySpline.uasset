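; BP_MySpline is a spline actor that lays a configurable mesh along its Spline component, with no active runtime logic.
; The Construction Script adds one SplineMeshComponent per segment between neighboring spline points, applying the chosen mesh, material, uniform cross-section scale and forward axis.
; Each segment takes its start and end from the local-space locations and tangents of its two points, so the mesh bends along the curve.
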(fn `UserConstructionScript`
  (bind _spline (`self.Spline`))
  (bind _meshscale_ (`self.MeshScale `))
  (for _index (range (+ (- (`SplineComponent.GetNumberOfSplinePoints` _spline) 2) 1))
    (bind _returnvalue (`AddComponent|NODE_AddSplineMeshComponent-0`))
    (`StaticMeshComponent.SetStaticMesh` _returnvalue (`self.New Mesh`))
    (`PrimitiveComponent.SetMaterial` _returnvalue 0 (`self.Material`))
    (`SplineMeshComponent.SetStartScale` _returnvalue (`KismetMathLibrary.MakeVector2D` _meshscale_ _meshscale_) true)
    (`SplineMeshComponent.SetEndScale` _returnvalue (`KismetMathLibrary.MakeVector2D` _meshscale_ _meshscale_) true)
    (`SplineMeshComponent.SetForwardAxis` _returnvalue (`self.In Forward Axis`) true)
    (bind (_location _tangent) (`SplineComponent.GetLocationAndTangentAtSplinePoint` _spline _index "Local"))
    (bind (_location_2 _tangent_2) (`SplineComponent.GetLocationAndTangentAtSplinePoint` _spline (+ _index 1) "Local"))
    (`SplineMeshComponent.SetStartAndEnd` _returnvalue _location _tangent _location_2 _tangent_2 true)))